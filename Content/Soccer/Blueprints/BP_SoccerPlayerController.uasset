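; Player controller for the soccer game that sets up MVVM car-selection data and opens the team selector at startup.
; The construction script lists six car IDs; BeginPlay registers a CarListVM globally and adds one entry per ID through CreateCarViewModelByID.
; That function's body is empty here, while CreateCarViewModelByID_0 copies car stats into a new CarVM.
; Finally, it shows WBP_Main_Team with mouse cursor and UI-only input.
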(event `self.ReceiveBeginPlay`
  (`|ExecutionSequence`
    (:`then_0`
      (bind _returnvalue (`|GenericCreateObject` "/Game/Soccer/Blueprints/ViewModels/CarListVM.CarListVM_C"))
      (bind _output_get (set `self.CarListVM` _returnvalue))
      (`MVVMViewModelCollectionObject.AddViewModelInstance` (`MVVMGameSubsystem.GetViewModelCollection` (subsystem `MVVMGameSubsystem`)) (make `MVVMViewModelContext` "/Game/Soccer/Blueprints/ViewModels/CarListVM.CarListVM_C" "CarListVM") _output_get))
    (:`then_1`
      (for _array_element (`self.CarIDs`)
        (bind _car_vm (`self.CreateCarViewModelByID` _array_element))
        (`KismetArrayLibrary.Array_Add` (`/Game/Soccer/Blueprints/ViewModels/CarListVM.CarVMs` (`self.CarListVM`)) _car_vm)))
    (:`then_2`
      (`self.OpenTeamSelector`))))

(event `OpenTeamSelector`
  (bind _returnvalue (`|GenericCreateObject` "/Game/Soccer/Blueprints/Widgets/WBP_Main_Team.WBP_Main_Team_C"))
  (`UserWidget.AddToViewport` _returnvalue 0)
  (set `self.bShowMouseCursor` true)
  (`WidgetBlueprintLibrary.SetInputMode_UIOnlyEx` self _returnvalue))

(fn `CreateCarViewModelByID`
  (params (`Car ID` :type "/Game/Soccer/Blueprints/BP_CarID Object Reference"))
  (returns (`Car VM` :type "/Game/Soccer/Blueprints/ViewModels/CarVM Object Reference"))
  (return null))

(fn `CreateCarViewModelByID_0`
  (params (`Car ID` :type "/Game/Soccer/Blueprints/BP_CarID Object Reference"))
  (returns (`Car VM` :type "/Game/Soccer/Blueprints/ViewModels/CarVM Object Reference"))
  (locals (CreatedCarVM :type "/Game/Soccer/Blueprints/ViewModels/CarVM Object Reference"))
  (bind _returnvalue (`|GenericCreateObject` "/Game/Soccer/Blueprints/ViewModels/CarVM.CarVM_C"))
  (bind _output_get (set `local.CreatedCarVM` _returnvalue))
  (set `/Game/Soccer/Blueprints/ViewModels/CarVM.Name` (`/Game/Soccer/Blueprints/BP_CarID.Name` (`local.Car ID`)) _output_get)
  (set `/Game/Soccer/Blueprints/ViewModels/CarVM.Icon` (`/Game/Soccer/Blueprints/BP_CarID.Icon` (`local.Car ID`)) (`local.CreatedCarVM`))
  (set `/Game/Soccer/Blueprints/ViewModels/CarVM.Length` (`/Game/Soccer/Blueprints/BP_CarID.Length` (`local.Car ID`)) (`local.CreatedCarVM`))
  (set `/Game/Soccer/Blueprints/ViewModels/CarVM.Width` (`/Game/Soccer/Blueprints/BP_CarID.Width` (`local.Car ID`)) (`local.CreatedCarVM`))
  (set `/Game/Soccer/Blueprints/ViewModels/CarVM.Height` (`/Game/Soccer/Blueprints/BP_CarID.Height` (`local.Car ID`)) (`local.CreatedCarVM`))
  (set `/Game/Soccer/Blueprints/ViewModels/CarVM.SurfaceArea` (`/Game/Soccer/Blueprints/BP_CarID.SurfaceArea` (`local.Car ID`)) (`local.CreatedCarVM`))
  (set `/Game/Soccer/Blueprints/ViewModels/CarVM.0% Boosting` (`/Game/Soccer/Blueprints/BP_CarID.0% Boosting` (`local.Car ID`)) (`local.CreatedCarVM`))
  (set `/Game/Soccer/Blueprints/ViewModels/CarVM.100% Boosting` (`/Game/Soccer/Blueprints/BP_CarID.100% Boosting` (`local.Car ID`)) (`local.CreatedCarVM`))
  (set `/Game/Soccer/Blueprints/ViewModels/CarVM.TurningAverage` (`/Game/Soccer/Blueprints/BP_CarID.TurningAverage` (`local.Car ID`)) (`local.CreatedCarVM`))
  (set `/Game/Soccer/Blueprints/ViewModels/CarVM.Is Selected?` false (`local.CreatedCarVM`))
  (return (`local.CreatedCarVM`)))

(fn `UserConstructionScript`
  (`KismetArrayLibrary.Array_Clear` (`self.CarIDs`))
  (`KismetArrayLibrary.Array_Add` (`self.CarIDs`) "/Game/Soccer/Data/CarID/CarID_Octane.CarID_Octane")
  (`KismetArrayLibrary.Array_Add` (`self.CarIDs`) "/Game/Soccer/Data/CarID/CarID_Dominus.CarID_Dominus")
  (`KismetArrayLibrary.Array_Add` (`self.CarIDs`) "/Game/Soccer/Data/CarID/CarID_Breakout.CarID_Breakout")
  (`KismetArrayLibrary.Array_Add` (`self.CarIDs`) "/Game/Soccer/Data/CarID/CarID_Gizmo.CarID_Gizmo")
  (`KismetArrayLibrary.Array_Add` (`self.CarIDs`) "/Game/Soccer/Data/CarID/CarID_DeLorean.CarID_DeLorean")
  (`KismetArrayLibrary.Array_Add` (`self.CarIDs`) "/Game/Soccer/Data/CarID/CarID_Paladin.CarID_Paladin"))