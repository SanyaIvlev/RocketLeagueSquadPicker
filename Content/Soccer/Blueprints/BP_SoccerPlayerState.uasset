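; Player state for the soccer game, holding a player's team and three chosen cars (center, left, right).
; On BeginPlay it creates empty car ID objects and registers a PlayerTeamVM in the global MVVM collection.
; UpdateTeam sets the viewmodel's blue/orange flags and, for a defined team, has player controller 0 process team slot viewmodels.
; Car OnRep handlers are empty; Tick debug-prints the center car's name.
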(event `self.ReceiveBeginPlay`
  (`self.CreateEmptyCarIDs`)
  (`self.TryMakeTeamVM`))

(event `TryMakeTeamVM`
  (if (not (`self.IsTeamVMCreated?`))
    (bind _returnvalue (`|GenericCreateObject` "/Game/Soccer/Blueprints/ViewModels/PlayerTeamVM.PlayerTeamVM_C"))
    (bind _output_get (set `self.PlayerTeamVM` _returnvalue))
    (bind _returnvalue_2 (`MVVMViewModelCollectionObject.AddViewModelInstance` (`MVVMGameSubsystem.GetViewModelCollection` (subsystem `MVVMGameSubsystem`)) (make `MVVMViewModelContext` "/Game/Soccer/Blueprints/ViewModels/PlayerTeamVM.PlayerTeamVM_C" "PlayerTeamVM") _output_get))
    (set `self.IsTeamVMCreated?` _returnvalue_2)))

(event `UpdateTeam`
  (params (`New Team` :type "GameplayTag Structure"))
  (set `self.Team` `New Team`)
  (set `/Game/Soccer/Blueprints/ViewModels/PlayerTeamVM.IsBlue?` (== (`self.Team`) (struct :`TagName` "Team.Blue")) (`self.PlayerTeamVM`))
  (set `/Game/Soccer/Blueprints/ViewModels/PlayerTeamVM.IsOrange?` (== (`self.Team`) (struct :`TagName` "Team.Orange")) (`self.PlayerTeamVM`))
  (if (!= (`self.Team`) (struct :`TagName` "Team.Undefined"))
    (bind _asbp_soccer_player_controller (cast `/Game/Soccer/Blueprints/BP_SoccerPlayerController` (`GameplayStatics.GetPlayerController` 0)))
    (`/Game/Soccer/Blueprints/BP_SoccerPlayerController.ClientRPC_ProcessPlayerTeamSlotsVM` _asbp_soccer_player_controller)))

(event `self.ReceiveTick`
  (params (DeltaSeconds :type "Float (single-precision)"))
  (`KismetSystemLibrary.PrintString` (`KismetTextLibrary.Conv_TextToString` (`/Game/Soccer/Blueprints/BP_CarID.Name` (`self.ChosenCenterCar`))) true true (struct :`G` 0.66 :`B` 1.0 :`A` 1.0) DeltaSeconds))

(fn `CreateEmptyCarIDs`
  (`|ExecutionSequence`
    (:`then_0`
      (bind _returnvalue (`|GenericCreateObject` "/Game/Soccer/Blueprints/BP_CarID.BP_CarID_C"))
      (set `self.ChosenCenterCar` _returnvalue))
    (:`then_1`
      (bind _returnvalue_2 (`|GenericCreateObject` "/Game/Soccer/Blueprints/BP_CarID.BP_CarID_C"))
      (set `self.ChosenLeftCar` _returnvalue_2))
    (:`then_2`
      (bind _returnvalue_3 (`|GenericCreateObject` "/Game/Soccer/Blueprints/BP_CarID.BP_CarID_C"))
      (set `self.ChosenRightCar` _returnvalue_3))))

(fn `OnRep_ChosenCenterCar`)

(fn `OnRep_ChosenLeftCar`)

(fn `OnRep_ChosenRightCar`)

(fn `UserConstructionScript`)