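; TeamSlotsVM is a soccer view model that groups the center, left and right car slot view models of a team.
; On initialization it binds event delegates to each slot's OnEquippedCarChanged dispatcher.
; BroadcastChangeInEquipment fires the team-level OnSlotsEquipmentChanged dispatcher, giving listeners a single notification point for equipment changes.
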(event `OnInitialized`
  (add `/Game/Soccer/Blueprints/ViewModels/CarPositionVM.OnEquippedCarChanged` (`self.CenterCarSlotVM`) (`|CreateDelegate` :!event `BroadcastChangeInEquipment`))
  (add `/Game/Soccer/Blueprints/ViewModels/CarPositionVM.OnEquippedCarChanged` (`self.LeftCarSlotVM`) (`|CreateDelegate` :!event `BroadcastChangeInEquipment`))
  (add `/Game/Soccer/Blueprints/ViewModels/CarPositionVM.OnEquippedCarChanged` (`self.RightCarSlotVM`) (`|CreateDelegate` :!event `BroadcastChangeInEquipment`)))

(event `BroadcastChangeInEquipment`
  (`self.OnSlotsEquipmentChanged` self))